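; FallTrigger is a trigger actor that registers a death when the player character falls into it.
; On BeginPlay it binds to its own begin-overlap event and ignores actors that are not MyCharacter.
; It compares world Z positions, and only when the character is above the trigger does it increment NumDeaths and play the Hurt sound at the character's location.
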(event Custom|OnActorBeginOverlap_Event_0
  (params (OtherActor :type Actor%20Object%20Reference))
  (bind _asmy_character (Utilities|Casting|CastToMyCharacter OtherActor))
  (Math|Float|CompareFloat (.Z (Math|Vector|BreakVector (Transformation|GetWorldLocation _asmy_character))) (.Z (Math|Vector|BreakVector (Transformation|GetWorldLocation)))
    (:>
      (Variables|/Game/Blueprints/MyCharacter.MyCharacter_C|SetnumDeaths _asmy_character (+ (Variables|/Game/Blueprints/MyCharacter.MyCharacter_C|GetnumDeaths _asmy_character) 1))
      (Audio|PlaySoundatLocation "/Game/Sounds/Hurt.Hurt" (Transformation|GetWorldLocation _asmy_character)))))

(event EventBeginPlay
  (EventDispatchers|AssignOnActorBeginOverlap (delegate Custom|OnActorBeginOverlap_Event_0)))

(fn ConstructionScript)